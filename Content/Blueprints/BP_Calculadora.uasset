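; BP_Calculadora is a calculator Blueprint that prints arithmetic and a comparison of its variables A and B on BeginPlay.
; A Sequence prints the sum, difference, product and quotient in one colored string, then the comparison result twice.
; NumberComparizon uses nested branches to store and return a Spanish less, equal or greater message in ResultadoComparacion.
; The division divides A by a literal zero, despite its A/B label.
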(event `self.ReceiveBeginPlay`
  (bind _a (`self.A`))
  (bind _b (`self.B`))
  (`|ExecutionSequence`
    (:`then_0`
      ;[0 0 0 0.5] Calculos
      (`KismetSystemLibrary.PrintString` (`KismetStringLibrary.Concat_StrStr` "La suma de A+B= " (`KismetStringLibrary.Conv_IntToString` (+ _a _b)) " | " "La resta de A-B= " (`KismetStringLibrary.Conv_IntToString` (- _a _b)) " | " "La Multiplicacion de A*B= " (`KismetStringLibrary.Conv_IntToString` (* _a _b)) " | " "La division de A/B= " (`KismetStringLibrary.Conv_DoubleToString` (/ _a 0))) true true (struct :`G` 0.573076 :`B` 1.0 :`A` 1.0) 20.0))
    (:`then_1`
      (bind _result (`self.NumberComparizon` (`self.A`) (`self.B`)))
      (`KismetSystemLibrary.PrintString` _result true true (struct :`R` 0.301178 :`G` 1.0 :`A` 1.0) 6.0))
    (:`then_2`
      ;[0 0 0 0.5] Imprimir el Resultado de la comparacion
      (`KismetSystemLibrary.PrintString` (`self.Resultado Comparacion`) true true (struct :`R` 1.0 :`B` 0.269484 :`A` 1.0) 20.0))))

(fn `NumberComparizon`
  (params (InputA :type Integer) (InputB :type Integer))
  (returns (Result :type String))
  ;[0 0 0 0.5] Comparacion
  (if (< InputA InputB)
    (set `self.Resultado Comparacion` "A es menor que B")
    (elif (== InputA InputB)
      (set `self.Resultado Comparacion` "A y B son iguales")
      (else
        (set `self.Resultado Comparacion` "A es mayor que B"))))
  (return (`self.Resultado Comparacion`)))

(fn `UserConstructionScript`)