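; BP_Moneda is a coin pickup that spins and is collected when the player pawn touches its sphere.
; A proximity collision speeds up the rotating movement while the player pawn is near and slows it again on exit.
; On pickup it calls ImprimirMoneda on GM_MyGameMode, plays an explosion sound and particle effect, then destroys itself, or prints an error if the game mode cast fails.
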(event `self.Sphere.OnComponentBeginOverlap`
  (params (OverlappedComponent :type "PrimitiveComponent Object Reference") (OtherActor :type "Actor Object Reference") (OtherComp :type "PrimitiveComponent Object Reference") (OtherBodyIndex :type Integer) (bFromSweep :type Boolean) (SweepResult :type "HitResult Structure (by ref)"))
  (if (== OtherActor (`GameplayStatics.GetPlayerPawn` 0))
    (bind _asgm_my_game_mode (cast `/Game/Core/GM_MyGameMode` (`GameplayStatics.GetGameMode`))
      (:`then`
        (`/Game/Core/GM_MyGameMode.Imprimir Moneda` _asgm_my_game_mode)
        (`|ExecutionSequence`
          (:`then_0`
            (`GameplayStatics.PlaySound2D` "/Game/StarterContent/Audio/Explosion01.Explosion01" 1.0 1.0 0.0 null null))
          (:`then_1`
            (`GameplayStatics.SpawnEmitterAtLocation` "/Game/StarterContent/Particles/P_Explosion.P_Explosion" (`self.K2_GetActorLocation` self)))
          (:`then_2`
            (`self.K2_DestroyActor`))))
      (:`CastFailed`
        (`KismetSystemLibrary.PrintString` "ERORR")))))

(event `self.ProximityCollision.OnComponentBeginOverlap`
  (params (OverlappedComponent :type "PrimitiveComponent Object Reference") (OtherActor :type "Actor Object Reference") (OtherComp :type "PrimitiveComponent Object Reference") (OtherBodyIndex :type Integer) (bFromSweep :type Boolean) (SweepResult :type "HitResult Structure (by ref)"))
  (if (== OtherActor (`GameplayStatics.GetPlayerPawn` 0))
    (set `RotatingMovementComponent.RotationRate` (struct :`Yaw` 560.0) (`self.RotatingMovement`))))

(event `self.ProximityCollision.OnComponentEndOverlap`
  (params (OverlappedComponent :type "PrimitiveComponent Object Reference") (OtherActor :type "Actor Object Reference") (OtherComp :type "PrimitiveComponent Object Reference") (OtherBodyIndex :type Integer))
  (if (== OtherActor (`GameplayStatics.GetPlayerPawn` 0))
    (set `RotatingMovementComponent.RotationRate` (struct :`Yaw` 180.0) (`self.RotatingMovement`))))

(fn `UserConstructionScript`)