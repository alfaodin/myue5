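; BP_Puerta is a door actor that slides open when the player enters its Collision volume and back when they leave.
; Overlap begin and end events check that the actor is the player pawn, then play or reverse the MovimientoPuerta timeline.
; Each timeline update feeds its track value to MoveDoor, which sets the Puerta component's relative location.
; Both events also print debug messages in Spanish.
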(event `self.Collision.OnComponentBeginOverlap`
  (params (OverlappedComponent :type "PrimitiveComponent Object Reference") (OtherActor :type "Actor Object Reference") (OtherComp :type "PrimitiveComponent Object Reference") (OtherBodyIndex :type Integer) (bFromSweep :type Boolean) (SweepResult :type "HitResult Structure (by ref)"))
  (if (`self.CheckIfActorIsPlayer` OtherActor)
    (`|ExecutionSequence`
      (:`then_0`
        (`KismetSystemLibrary.PrintString` "Ingreso del personaje"))
      (:`then_1`
        (bind (_direction _newtrack_0) (`Timeline|MovimientoPuerta` :!label _label)
          (:`Update`
            (`self.MoveDoor` _newtrack_0)))))))

(event `self.Collision.OnComponentEndOverlap`
  (params (OverlappedComponent :type "PrimitiveComponent Object Reference") (OtherActor :type "Actor Object Reference") (OtherComp :type "PrimitiveComponent Object Reference") (OtherBodyIndex :type Integer))
  (if (`self.CheckIfActorIsPlayer` OtherActor)
    (`|ExecutionSequence`
      (:`then_0`
        (goto _label :!via `Reverse`))
      (:`then_1`
        (`KismetSystemLibrary.PrintString` "Salio del personaje")))))

(fn `CheckIfActorIsPlayer`
  (params (Actor :type "Object Object Reference"))
  (returns (IsPlayer :type Boolean))
  (return (== Actor (`GameplayStatics.GetPlayerPawn` 0))))

(fn `MoveDoor`
  (params (NewLocation_X :type "Float (double-precision)"))
  (`SceneComponent.K2_SetRelativeLocation` (`self.Puerta`) (`KismetMathLibrary.MakeVector` NewLocation_X) false false))

(fn `UserConstructionScript`)